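; Enemy AI character that fights via a combat system component, with an overhead health bar and an experience reward on death.
; Construction wires up its stats and combat components; Attack starts the combat component's attack and returns the attack speed.
; A looping timer turns the health bar toward the player camera.
; Death hides the bar, ragdolls the mesh, detaches the controller, plays a sound, destroys the actor after a delay and grants the player experience.
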(event EventOnCharacterDeath
  (Utilities|FlowControl|Sequence
    (:then_0
      (CallFunction|HideHealthbar)
      (CallFunction|DeathPhysics))
    (:then_1
      (Audio|PlaySoundatLocation "/Game/Audio/Combat/SC_Death.SC_Death" (Transformation|GetActorLocation) "0, 0, 0" 1.0 1.0 0.0 0 0 0 0))
    (:then_2
      (Utilities|FlowControl|Delay 1e+01)
      (Actor|DestroyActor))
    (:then_3
      (CallFunction|GiveExperiencetoPlayer))))

(event EventBeginPlay
  (Utilities|Time|SetTimerbyFunctionName 0 "SetHealthbarRotation" 0.05 true))

(fn ConstructionScript
  (Class|EnemyCharacter|SetCharacterStats (Variables|Default|GetBP_CharacterStats1))
  (Class|EnemyCharacter|SetCombatSystem (Variables|Default|GetBP_CombatSystem1)))

(fn SetHealthbarRotation
  (bind _health_bar_widget (Variables|Default|GetHealth%20Bar%20Widget))
  (Transformation|SetWorldRotation _health_bar_widget (Math|Rotator|FindLookatRotation (Transformation|GetWorldLocation _health_bar_widget) (Transformation|GetWorldLocation (Variables|/Script/Engine.PlayerCameraManager|GetTransformComponent (Game|GetPlayerCameraManager 0)))) false false))

(fn HideHealthbar
  (bind _aswbp_enemy_hud (Utilities|Casting|CastToWBP_EnemyHUD (UserInterface|GetWidget (Variables|Default|GetHealth%20Bar%20Widget))))
  (Variables|/Script/UMG.Widget|SetRenderOpacity (Variables|/Game/UI/InGameHUD/WBP_EnemyHUD.WBP_EnemyHUD_C|GetHealthBar _aswbp_enemy_hud) 0.0))

(fn DeathPhysics
  (Pawn|Components|CharacterMovement|DisableMovement (Variables|Character|GetCharacterMovement))
  (Collision|SetCollisionEnabled (Variables|Default|GetCapsuleComponent) "PhysicsOnly")
  (Physics|SetSimulatePhysics (Variables|Character|GetMesh) true)
  (Class|Pawn|DetachfromControllerPendingDestroy)
  (Utilities|Array|Clear (Variables|Default|GetTags)))

(fn GiveExperiencetoPlayer
  (bind _asbp_third_person_character_1 (Utilities|Casting|CastToBP_ThirdPersonCharacter1 (Pawn|GetControlledPawn (Game|GetPlayerController 0)))
    (:then
      (Class|LicentaRPGCharacter|GainExperience _asbp_third_person_character_1 (Variables|Default|GetExperienceGiven)))
    (:CastFailed
      (Development|PrintString "Failed to cast as BP_ThirdPersonCharacter in GiveExperienceToPlayer in BP_EnemyAI"))))

(fn Attack
  (Class|CombatSystem|StartAttack (Variables|Default|GetBP_CombatSystem1))
  (return (Variables|Default|GetAttackSpeed)))